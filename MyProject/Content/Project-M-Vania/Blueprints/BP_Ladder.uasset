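; BP_Ladder is a 2D ladder actor that lets BP_Player_Placeholder climb while inside its Box trigger.
; Its construction script stacks non-colliding Paper sprites at RungOffset intervals over the height between LadderBottom and LadderTop, then scales and raises the Box from that height.
; Box overlaps set the player's CanClimb on entry, and clear it and call ClimbingEvent on exit.
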(event `self.Box.OnComponentBeginOverlap`
  (params (OverlappedComponent :type "PrimitiveComponent Object Reference") (OtherActor :type "Actor Object Reference") (OtherComp :type "PrimitiveComponent Object Reference") (OtherBodyIndex :type Integer) (bFromSweep :type Boolean) (SweepResult :type "HitResult Structure (by ref)"))
  (bind _asbp_player_placeholder (cast `/Game/Project-M-Vania/Blueprints/BP_Player_Placeholder` OtherActor))
  (set `/Game/Project-M-Vania/Blueprints/BP_Player_Placeholder.canClimb` true _asbp_player_placeholder))

(event `self.Box.OnComponentEndOverlap`
  (params (OverlappedComponent :type "PrimitiveComponent Object Reference") (OtherActor :type "Actor Object Reference") (OtherComp :type "PrimitiveComponent Object Reference") (OtherBodyIndex :type Integer))
  (bind _asbp_player_placeholder (cast `/Game/Project-M-Vania/Blueprints/BP_Player_Placeholder` OtherActor))
  (set `/Game/Project-M-Vania/Blueprints/BP_Player_Placeholder.canClimb` false _asbp_player_placeholder)
  (`/Game/Project-M-Vania/Blueprints/BP_Player_Placeholder.ClimbingEvent` _asbp_player_placeholder))

(fn `UserConstructionScript`
  (bind _rungoffset (`self.RungOffset`))
  (bind _box (`self.Box`))
  (bind (_returnvalue_x _returnvalue_y _returnvalue_z) (`KismetMathLibrary.BreakVector` (- (`self.LadderTop`) (`self.LadderBottom`))))
  (bind _returnvalue (/ _returnvalue_z 2.0))
  (for _index (range (+ (`KismetMathLibrary.FTrunc` (/ _returnvalue_z _rungoffset)) 1))
    (bind _returnvalue_2 (`AddComponent|NODE_AddPaperSpriteComponent-0` :`RelativeTransform` (`KismetMathLibrary.MakeTransform` (`KismetMathLibrary.MakeVector` 0.0 0.0 (* _index _rungoffset)))))
    (`PaperSpriteComponent.SetSprite` _returnvalue_2 (`self.LadderSprite`))
    (`PrimitiveComponent.SetCollisionEnabled` _returnvalue_2 "NoCollision"))
  (`SceneComponent.SetRelativeScale3D` _box (`KismetMathLibrary.MakeVector` 1.0 1.0 _returnvalue))
  (`SceneComponent.K2_AddRelativeLocation` _box (`KismetMathLibrary.MakeVector` 0.0 0.0 _returnvalue) false false))